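; BP_Penis is a three-part penis actor with tinted materials and an optional BP_Hut spawned onto its End at BeginPlay.
; Tick snaps Base and End to Middle's skeletal sockets.
; Capsule overlaps play audio and trigger a soft Touch, bursting Niagara only without a hut, while a hard Touch detaches the hut and always bursts.
; SetLength swaps Middle's mesh and enables physics but is unused here; click handlers only print debug text.
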(event `Lose Hut`
  (bind _hut (`self.Hut`))
  (`/Engine/EditorBlueprintResources/StandardMacros.IsValid` _hut
    (:`Is Valid`
      (`self.K2_DetachFromActor` _hut "KeepWorld" "KeepWorld" "KeepWorld")
      (`/Game/TheBestGame/Blueprints/BP_Hut.Detach` _hut)
      (set `self.Hut` null))))

(event `self.ReceiveBeginPlay`
  (if (`self.bHut`)
    (bind _returnvalue (`|SpawnActorFromClass` "/Game/TheBestGame/Blueprints/BP_Hut.BP_Hut_C" (`KismetMathLibrary.MakeTransform` (0.0 0.0 0.0)) "Undefined" "OverrideRootScale" null (struct :`B` 129 :`G` 60 :`R` 165) null))
    (set `self.Hut` _returnvalue)
    (`self.K2_AttachToComponent` _returnvalue (`self.End`) "hut" "KeepRelative" "KeepRelative" "KeepRelative" true)))

(event `self.ReceiveTick`
  (params (DeltaSeconds :type "Float (single-precision)"))
  (bind _middle (`self.Middle`))
  (bind _end (`self.End`))
  (bind _base (`self.Base`))
  (bind (_returnvalue_location _returnvalue_rotation) (`KismetMathLibrary.BreakTransform` (`SceneComponent.GetSocketTransform` _middle "startSocket" "RTS_World")))
  (bind (_returnvalue_location_2 _returnvalue_rotation_2) (`KismetMathLibrary.BreakTransform` (`SceneComponent.GetSocketTransform` _middle "endSocket" "RTS_World")))
  (`/Engine/EditorBlueprintResources/StandardMacros.IsValid` _base
    (:`Is Valid`
      (`SceneComponent.K2_SetWorldTransform` _base (`KismetMathLibrary.MakeTransform` _returnvalue_location _returnvalue_rotation (`SceneComponent.K2_GetComponentScale` _base)) false false)
      (`/Engine/EditorBlueprintResources/StandardMacros.IsValid` _end
        (:`Is Valid`
          (`SceneComponent.K2_SetWorldTransform` _end (`KismetMathLibrary.MakeTransform` _returnvalue_location_2 _returnvalue_rotation_2 (`SceneComponent.K2_GetComponentScale` _end)) false false))))))

(event `self.Capsule.OnComponentBeginOverlap`
  (params (OverlappedComponent :type "PrimitiveComponent Object Reference") (OtherActor :type "Actor Object Reference") (OtherComp :type "PrimitiveComponent Object Reference") (OtherBodyIndex :type Integer) (bFromSweep :type Boolean) (SweepResult :type "HitResult Structure (by ref)"))
  (`self.Touch` false)
  (`AudioComponent.Play` (`self.AudioCurveSource`) 0.0))

(event `Touch`
  (params (Hard :type Boolean))
  (bind _niagara (`self.Niagara`))
  (if Hard
    (`self.Lose Hut`)
    (`ActorComponent.Activate` _niagara false :!label _label)
    (`KismetSystemLibrary.Delay` 0.2)
    (`ActorComponent.Deactivate` _niagara)
    (elif (not (`KismetSystemLibrary.IsValid` (`self.Hut`)))
      (goto _label))))

(event `self.Middle.OnComponentHit`
  (params (HitComponent :type "PrimitiveComponent Object Reference") (OtherActor :type "Actor Object Reference") (OtherComp :type "PrimitiveComponent Object Reference") (NormalImpulse :type "Vector Structure") (Hit :type "HitResult Structure (by ref)"))
  (`KismetSystemLibrary.PrintString` "Hello"))

(event `self.Middle.OnClicked`
  (params (TouchedComponent :type "PrimitiveComponent Object Reference") (ButtonPressed :type "Key Structure"))
  (`KismetSystemLibrary.PrintString` "Click" :!label _label_2))

(event `self.Middle.OnInputTouchBegin`
  (params (FingerIndex :type "ETouchIndex Enum" :default "Touch1") (TouchedComponent :type "PrimitiveComponent Object Reference"))
  (goto _label_2))

(event `self.End.OnClicked`
  (params (TouchedComponent :type "PrimitiveComponent Object Reference") (ButtonPressed :type "Key Structure"))
  (goto _label_2))

(event `self.Base.OnClicked`
  (params (TouchedComponent :type "PrimitiveComponent Object Reference") (ButtonPressed :type "Key Structure"))
  (goto _label_2))

(event `HandleControllerClick`
  (goto _label_2))

(event `self.Capsule.OnBeginCursorOver`
  (params (TouchedComponent :type "PrimitiveComponent Object Reference")))

(fn `SetLength`
  (params (Selection :type Integer))
  (locals (NewLocalVar_0 :type Name :default "Armature_006"))
  (bind _middle (`self.Middle`))
  (switch `int` Selection
    (:`0`
      _)
    (:`1`
      _)
    (:`2`
      _)
    (:`3`
      _))
  (`SkinnedMeshComponent.SetSkinnedAssetAndUpdate` (`self.Middle`) (`|GetArrayItem` (`self.Centers`) Selection) true)
  (`SkeletalMeshComponent.SetAllBodiesBelowSimulatePhysics` _middle "Bone" true true)
  (`SkeletalMeshComponent.SetAllBodiesPhysicsBlendWeight` _middle 1.0 false)
  (`PrimitiveComponent.SetCollisionEnabled` (`self.Middle`) "PhysicsOnly")
  (`PrimitiveComponent.SetCollisionEnabled` _middle "PhysicsOnly"))

(fn `UserConstructionScript`
  (bind _returnvalue (`KismetMathLibrary.Conv_ColorToLinearColor` (`self.Color`)))
  (`|ExecutionSequence`
    (:`then_1`
      (bind _returnvalue_2 (`PrimitiveComponent.CreateDynamicMaterialInstance` (`self.Middle`) 0 null "None"))
      (bind _returnvalue_3 (`PrimitiveComponent.CreateDynamicMaterialInstance` (`self.Base`) 0 null "None"))
      (bind _returnvalue_4 (`PrimitiveComponent.CreateDynamicMaterialInstance` (`self.End`) 0 null "None"))
      (`MaterialInstanceDynamic.SetVectorParameterValue` _returnvalue_2 "Color" _returnvalue)
      (`MaterialInstanceDynamic.SetVectorParameterValue` _returnvalue_3 "Color" _returnvalue)
      (`MaterialInstanceDynamic.SetVectorParameterValue` _returnvalue_4 "Color" _returnvalue))))