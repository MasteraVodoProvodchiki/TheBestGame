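; Spawner actor that keeps a box volume, sized by Extent in the construction script, populated with BP_Penis actors up to Amount.
; It optionally fills on BeginPlay, then a looping timer adds one while below the cap, with OnDestroyed bindings decrementing the count.
; Each spawn gets a random position, rotation, scale, color and Hut flag.
; A random switch picks among four variant classes, making s4 the rarest.
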(event `self.ReceiveBeginPlay`
  ;[1 1 1] Spawn Every Time
  (`KismetSystemLibrary.K2_SetTimerDelegate` (delegate `OnTimer`) (`self.SpawTime`) true)
  ;[1 1 1] Fill on Start
  (if (`self.AutoFill`)
    (for _ (range (+ (`self.Amount`) 1))
      (`self.Create Penis`))))

(event `OnTimer`
  ;[1 1 1] Spawn Every Time
  (if (< (`self.Count`) (`self.Amount`))
    (`self.Create Penis`)))

(event `Create Penis`
  (bind _extent (`self.Extent`))
  (bind _returnvalue (`SceneComponent.K2_GetComponentLocation` (`self.DefaultSceneRoot`)))
  (bind (_returnvalue_x _returnvalue_y _returnvalue_z) (`KismetMathLibrary.BreakVector` (- _returnvalue _extent)))
  (bind (_returnvalue_x_2 _returnvalue_y_2 _returnvalue_z_2) (`KismetMathLibrary.BreakVector` (+ _returnvalue _extent)))
  (bind _penis (`self.Spawn Penis` (`KismetMathLibrary.MakeTransform` (`KismetMathLibrary.MakeVector` (`KismetMathLibrary.RandomFloatInRange` _returnvalue_x _returnvalue_x_2) (`KismetMathLibrary.RandomFloatInRange` _returnvalue_y _returnvalue_y_2) (`KismetMathLibrary.RandomFloatInRange` _returnvalue_z _returnvalue_z_2)) (`KismetMathLibrary.RandomRotator` false) (`KismetMathLibrary.Conv_DoubleToVector` (`KismetMathLibrary.RandomFloatInRange` 0.3 0.5)))))
  (`/Engine/EditorBlueprintResources/StandardMacros.IncrementInt` (`self.Count`)
    (:`  `
      (add `self.OnDestroyed` _penis (delegate `OnDestroyed_Event_0`)))))

(event `OnDestroyed_Event_0` :!signature `self.OnDestroyed`
  (params (DestroyedActor :type "Actor Object Reference"))
  (`/Engine/EditorBlueprintResources/StandardMacros.DecrementInt` (`self.Count`)))

(fn `Spawn Penis`
  (params (Transofrm :type "Transform Structure"))
  (returns (Penis :type "/Game/TheBestGame/Blueprints/BP_Penis Object Reference"))
  (locals (Output :type "/Game/TheBestGame/Blueprints/BP_Penis Object Reference"))
  (bind _colors (`self.Colors`))
  (bind _returnvalue (< (`KismetMathLibrary.RandomFloat`) 0.3))
  (bind _output (`|GetArrayItem` _colors (`KismetMathLibrary.RandomIntegerInRange` 0 (- (`KismetArrayLibrary.Array_Length` _colors) 1))))
  (switch `int` (`KismetMathLibrary.RandomIntegerInRange` 0 9)
    (:`0`
      (bind _returnvalue_2 (`|SpawnActorFromClass` "/Game/TheBestGame/Blueprints/BP_Penis_s1.BP_Penis_s1_C" Transofrm "Undefined" "OverrideRootScale" null _output 0 _returnvalue null :!label _label))
      (set `local.Output` _returnvalue_2))
    (:`1`
      (goto _label))
    (:`2`
      (goto _label))
    (:`3`
      (bind _returnvalue_3 (`|SpawnActorFromClass` "/Game/TheBestGame/Blueprints/BP_Penis_s2.BP_Penis_s2_C" Transofrm "Undefined" "OverrideRootScale" null _output 1 _returnvalue null :!label _label_2))
      (set `local.Output` _returnvalue_3))
    (:`4`
      (goto _label_2))
    (:`5`
      (goto _label_2))
    (:`6`
      (bind _returnvalue_4 (`|SpawnActorFromClass` "/Game/TheBestGame/Blueprints/BP_Penis_s3.BP_Penis_s3_C" Transofrm "Undefined" "OverrideRootScale" null _output 2 _returnvalue null :!label _label_3))
      (set `local.Output` _returnvalue_4))
    (:`7`
      (goto _label_3))
    (:`8`
      (goto _label_3))
    (:`9`
      (bind _returnvalue_5 (`|SpawnActorFromClass` "/Game/TheBestGame/Blueprints/BP_Penis_s4.BP_Penis_s4_C" Transofrm "Undefined" "OverrideRootScale" null _output 3 _returnvalue null))
      (set `local.Output` _returnvalue_5)))
  (return (`local.Output`)))

(fn `UserConstructionScript`
  (`BoxComponent.SetBoxExtent` (`self.Box`) (`self.Extent`) true))