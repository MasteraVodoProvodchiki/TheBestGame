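; BP_Hut is a hut actor (by its name) with a randomly colored static mesh that can become a physics object.
; The construction script disables mesh collision and creates a dynamic material instance, setting its Color parameter to a random entry from the Colors array.
; The Detach event later enables query and physics collision and starts physics simulation on the mesh.
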(event `Detach`
  (bind _staticmesh (`self.StaticMesh`))
  (`PrimitiveComponent.SetCollisionEnabled` _staticmesh "QueryAndPhysics")
  (`PrimitiveComponent.SetSimulatePhysics` _staticmesh true))

(fn `UserConstructionScript`
  (bind _staticmesh (`self.StaticMesh`))
  (bind _colors (`self.Colors`))
  (`PrimitiveComponent.SetCollisionEnabled` _staticmesh "NoCollision")
  (bind _returnvalue (`PrimitiveComponent.CreateDynamicMaterialInstance` _staticmesh 0 null "None"))
  (bind _output_get (set `self.Color` (`|GetArrayItem` _colors (`KismetMathLibrary.RandomIntegerInRange` 0 (`KismetArrayLibrary.Array_LastIndex` _colors)))))
  (`MaterialInstanceDynamic.SetVectorParameterValue` _returnvalue "Color" (`KismetMathLibrary.Conv_ColorToLinearColor` _output_get)))